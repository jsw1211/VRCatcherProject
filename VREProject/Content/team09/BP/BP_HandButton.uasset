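; BP_HandButton is a pressable button that toggles the player's left-hand setting.
; Each ButtonComponent press flips IsLeftHand and updates the TextRender label, showing On when the flag becomes false and Off when true.
; It then writes the new value to the GI_Variables game instance.
; Glove visibility swap nodes are left unconnected and never run, and NewFunction is empty.
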(event `self.ButtonComponent.ButtonPressed`
  (params (ButtonState :type Boolean))
  (bind _returnvalue (`GameplayStatics.GetGameInstance`))
  (bind _islefthand (`self.IsLeftHand`))
  (bind _textrender (`self.TextRender`))
  (if (`self.IsLeftHand`)
    (`TextRenderComponent.K2_SetText` _textrender (`self.On`))
    (set `self.IsLeftHand` false)
    (bind _asgi_variables (cast `/Game/team09/BP/GI_Variables` _returnvalue))
    (set `/Game/team09/BP/GI_Variables.IsLeftHand?` _islefthand _asgi_variables)
    (else
      (`TextRenderComponent.K2_SetText` _textrender (`self.Off`))
      (set `self.IsLeftHand` true)
      (bind _asgi_variables_2 (cast `/Game/team09/BP/GI_Variables` _returnvalue))
      (set `/Game/team09/BP/GI_Variables.IsLeftHand?` _islefthand _asgi_variables_2))))

(fn `NewFunction`)

(fn `UserConstructionScript`
  (`parent.UserConstructionScript`))