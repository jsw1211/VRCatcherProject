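; BP_GameResultManager is an actor that records pitch results and catch-or-miss outcomes for a pitching and catching game.
; AddPitchResult and AddCatchOrMiss append to two separate arrays, which are both cleared on BeginPlay.
; PrintPitchResults dumps both arrays to screen with their indices, showing pitcher name, ball type and ball speed for each pitch, then each catch-or-miss text.
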(event `self.ReceiveBeginPlay`
  (`KismetArrayLibrary.Array_Clear` (`self.PitchResults`))
  (`KismetArrayLibrary.Array_Clear` (`self.Catch or Miss arr`)))

(event `Print Pitch Results`
  (for (_array_element _array_index) (`self.PitchResults`)
    (`KismetSystemLibrary.PrintString` (`KismetStringLibrary.Conv_NameToString` (break `/Game/team09/BP/Enum/ST_PitchResult` _array_element)))
    (`KismetSystemLibrary.PrintString` (`KismetStringLibrary.Conv_NameToString` (`.BallType_11_C151C0144383E1FA272B679D24C59041` (break `/Game/team09/BP/Enum/ST_PitchResult` _array_element))))
    (`KismetSystemLibrary.PrintString` (`KismetStringLibrary.Conv_DoubleToString` (`.BallSpeed_9_0943393949EFA9C475E22CA6AD7E267E` (break `/Game/team09/BP/Enum/ST_PitchResult` _array_element))))
    (`KismetSystemLibrary.PrintString` (`KismetStringLibrary.Conv_IntToString` _array_index)))
  (for (_array_element_2 _array_index_2) (`self.Catch or Miss arr`)
    (`KismetSystemLibrary.PrintText` _array_element_2)
    (`KismetSystemLibrary.PrintText` (`KismetTextLibrary.Conv_IntToText` _array_index_2))))

(fn `Add Catch or Miss`
  (params (`New Catch or Miss` :type Text))
  (`KismetArrayLibrary.Array_Add` (`self.Catch or Miss arr`) `New Catch or Miss`))

(fn `Add PitchResult`
  (params (`New Result` :type "/Game/team09/BP/Enum/ST_PitchResult Structure"))
  (`KismetArrayLibrary.Array_Add` (`self.PitchResults`) `New Result`))

(fn `UserConstructionScript`)