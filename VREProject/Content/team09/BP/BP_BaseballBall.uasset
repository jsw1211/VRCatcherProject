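; Baseball pitch actor that throws a chosen pitch type from one of three tagged pitchers to the catcher.
; ThrowingBall picks pitcher and spline by tag; StartMoving snaps the spline's end to the catcher's glove hand and plays the pitching animation.
; A Timeline moves the ball along the spline, its play rate derived from randomized km/h speed and spline length.
; On finish it reports the pitch to BP_GameResultManager; random target-scatter logic is disconnected.
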(event `self.ReceiveBeginPlay`)

(event `Throwing Ball`
  (params (`Current Pitch Type Index` :type Integer) (`Current Pitcher Index` :type Integer))
  (bind _characterselected (`self.CharacterSelected`))
  (bind _characterselected_2 (`self.CharacterSelected`))
  (set `self.Current Pitch Type Index` `Current Pitch Type Index`)
  (if (`KismetSystemLibrary.IsValid` _characterselected_2)
    (`self.SetActorHiddenInGame` _characterselected_2 true))
  (`KismetSystemLibrary.Delay` 0.1)
  (switch `int` `Current Pitcher Index`
    (:`0`
      (bind _pitcher_name (`self.Choose Pitcher Type` "hyunjin"))
      (set `self.Pitcher Name` _pitcher_name))
    (:`1`
      (bind _pitcher_name_2 (`self.Choose Pitcher Type` "seunghwan"))
      (set `self.Pitcher Name` _pitcher_name_2))
    (:`2`
      (bind _pitcher_name_3 (`self.Choose Pitcher Type` "ohtani"))
      (set `self.Pitcher Name` _pitcher_name_3)))
  (switch `int` (`self.Current Pitch Type Index`)
    (:`0`
      (set `self.Slider Speed Val` (`/Game/team09/character/BP_BaseCharacter.SliderSpeedVal` _characterselected))
      (bind _ball_type_name (`self.Choose Ball Type` "slider" "right"))
      (set `self.Ball Type Name` _ball_type_name))
    (:`1`
      (set `self.Curve Speed Val` (`/Game/team09/character/BP_BaseCharacter.CurveSpeedVal` _characterselected))
      (bind _ball_type_name_2 (`self.Choose Ball Type` "curve" "right"))
      (set `self.Ball Type Name` _ball_type_name_2))
    (:`2`
      (set `self.Fastball Speed Val` (`/Game/team09/character/BP_BaseCharacter.FastballSpeedVal` _characterselected))
      (bind _ball_type_name_3 (`self.Choose Ball Type` "fastball" "right"))
      (set `self.Ball Type Name` _ball_type_name_3))))

(event `StartMoving`
  (bind _characterselected (`self.CharacterSelected`))
  (bind _spline (`/Game/team09/BP/Spline/BP_SplineBase.Spline` (`self.SplineSelected`)))
  (bind _spline_2 (`/Game/team09/BP/Spline/BP_SplineBase.Spline` (`self.SplineSelected`)))
  (for _array_element (`self.SplinesSelected`)
    (bind _asbp_spline_base (cast `/Game/team09/BP/Spline/BP_SplineBase` _array_element))
    (set `self.SplineSelected` _asbp_spline_base)
    ; 스플라인의 마지막 점(공 도착지점) 변경
    (bind _asgi_variables (cast `/Game/team09/BP/GI_Variables` (`GameplayStatics.GetGameInstance`)))
    (if (`/Game/team09/BP/GI_Variables.IsLeftHand?` _asgi_variables)
      (bind _returnvalue (`GameplayStatics.GetActorOfClass` "/Game/team09/BP/BP_Catcher.BP_Catcher_C"))
      (set `self.Target Hand Location` (`self.K2_GetActorLocation` (`/Game/Platform/Core/Character/BP_VRCharacter.GraspingHandLeft` _returnvalue)))
      (else
        (bind _returnvalue_2 (`GameplayStatics.GetActorOfClass` "/Game/team09/BP/BP_Catcher.BP_Catcher_C"))
        (set `self.Target Hand Location` (`self.K2_GetActorLocation` (`/Game/Platform/Core/Character/BP_VRCharacter.GraspingHandRight` _returnvalue_2)))))
    (`SplineComponent.SetLocationAtSplinePoint` _spline (- (`SplineComponent.GetNumberOfSplinePoints` _spline) 1) (+ (`self.Target Hand Location`) (`KismetMathLibrary.MakeVector` 0.0 (* (`KismetMathLibrary.Cos` (`self.Angle`)) (`self.Distance`)) (* (`KismetMathLibrary.Sin` (`self.Angle`)) (`self.Distance`)))) "World" true)
    ; 투수 선택,애니메이션 재생
    (switch `name` (`self.Pitcher Name`)
      (:`hyunjin`
        (`self.SetActorHiddenInGame` _characterselected false)
        (bind _asbp_mh_hyun_jin (cast `/Game/team09/character/MH_HyunJin/BP_MH_HyunJin` _characterselected))
        (bind _returnvalue_3 (`GameplayStatics.GetActorOfClass` (`GameplayStatics.GetObjectClass` _asbp_mh_hyun_jin)))
        (`SkeletalMeshComponent.PlayAnimation` (`/Game/team09/character/MH_HyunJin/BP_MH_HyunJin.Body` _returnvalue_3) "/Game/team09/Animation/AS_Baseball_Pitching.AS_Baseball_Pitching" false))
      (:`seunghwan`
        (`self.SetActorHiddenInGame` _characterselected false)
        (bind _asbp_mh_seung_hwan (cast `/Game/team09/character/MH_SeungHwan/BP_MH_SeungHwan` _characterselected))
        (bind _returnvalue_4 (`GameplayStatics.GetActorOfClass` (`GameplayStatics.GetObjectClass` _asbp_mh_seung_hwan)))
        (`SkeletalMeshComponent.PlayAnimation` (`/Game/team09/character/MH_SeungHwan/BP_MH_SeungHwan.Body` _returnvalue_4) "/Game/team09/Animation/AS_Baseball_Pitching.AS_Baseball_Pitching" false))
      (:`ohtani`
        (`self.SetActorHiddenInGame` _characterselected false)
        (bind _asbp_mh_ohtani (cast `/Game/team09/character/MH_Ohtani/BP_MH_Ohtani` _characterselected))
        (bind _returnvalue_5 (`GameplayStatics.GetActorOfClass` (`GameplayStatics.GetObjectClass` _asbp_mh_ohtani)))
        (`SkeletalMeshComponent.PlayAnimation` (`/Game/team09/character/MH_Ohtani/BP_MH_Ohtani.Body` _returnvalue_5) "/Game/team09/Animation/AS_Baseball_Pitching.AS_Baseball_Pitching" false)))
    (`KismetSystemLibrary.Delay` 1.52)
    ; 최종 공 구속 결정
    (switch `int` (`self.Current Pitch Type Index`)
      (:`0`
        (set `self.NewSpeed` (+ (`self.Slider Speed Val`) (`self.DefaultSpeed`))))
      (:`1`
        (set `self.NewSpeed` (+ (`self.Curve Speed Val`) (`self.DefaultSpeed`))))
      (:`2`
        (set `self.NewSpeed` (+ (`self.Fastball Speed Val`) (`self.DefaultSpeed`)))))
    (bind _asgi_variables_2 (cast `/Game/team09/BP/GI_Variables` (`GameplayStatics.GetGameInstance`)))
    (if (`/Game/team09/BP/GI_Variables.IsProMod?` _asgi_variables_2)
      (set `self.ProModSpeed` 40.0)
      (else
        (set `self.ProModSpeed` 0.0)))
    (set `self.NewSpeed` (+ (`self.ProModSpeed`) (`self.NewSpeed`)))
    (set `self.NewSpeed` (`KismetMathLibrary.RandomFloatInRange` (* (`self.NewSpeed`) 0.9) (* (`self.NewSpeed`) 1.1)))
    (`KismetSystemLibrary.PrintText` (`KismetTextLibrary.Conv_DoubleToText` (`self.NewSpeed`) "HalfToEven" false true 1 324 0 2))
    (`PrimitiveComponent.SetCollisionEnabled` (`self.StaticMesh`) "QueryAndPhysics")
    ; 타임라인에 따라 실제 공 위치 이동
    (`TimelineComponent.SetPlayRate` (`self.Timeline`) (/ (* (* (/ (`self.NewSpeed`) 3.6) 100.0) (`TimelineComponent.GetTimelineLength` (`self.Timeline`))) (`SplineComponent.GetSplineLength` (`/Game/team09/BP/Spline/BP_SplineBase.Spline` (`self.SplineSelected`)))))
    (bind (_direction _newtrack_0) (`Timeline|Timeline` :!via `PlayFromStart`)
      (:`Update`
        (bind _returnvalue_6 (`KismetMathLibrary.Lerp` 0.0 (`SplineComponent.GetSplineLength` (`/Game/team09/BP/Spline/BP_SplineBase.Spline` (`self.SplineSelected`))) _newtrack_0))
        (`self.K2_SetActorLocationAndRotation` (`SplineComponent.GetLocationAtDistanceAlongSpline` _spline_2 _returnvalue_6 "World") (`SplineComponent.GetRotationAtDistanceAlongSpline` _spline_2 _returnvalue_6 "World")))
      (:`Finished`
        ;; 공 다 던졌음 호출
        (`KismetSystemLibrary.Delay` 1.0)
        (bind _returnvalue_7 (`GameplayStatics.GetActorOfClass` "/Game/team09/BP/BP_GameResultManager.BP_GameResultManager_C"))
        (`/Game/team09/BP/BP_GameResultManager.Add PitchResult` _returnvalue_7 (make `/Game/team09/BP/Enum/ST_PitchResult` (`self.Pitcher Name`) (`self.Ball Type Name`) (`self.NewSpeed`)))
        (set `self.Throwing all Completed` true)))))

(event `StopTimeline`
  (`Timeline|Timeline_0` :!via `Stop`))

(fn `Choose Ball Type`
  (params (`ball type` :type Name) (`left or right` :type Name))
  (returns (`ball type name` :type Name))
  (bind _ball_type (`self.Ball Type`))
  (set `self.Ball Type` `ball type`)
  (set `self.Left Or Right` `left or right`)
  (`KismetArrayLibrary.Array_Clear` (`self.SplinesSelected`))
  (bind _outactors (`GameplayStatics.GetAllActorsOfClass` "/Game/team09/BP/Spline/BP_SplineBase.BP_SplineBase_C"))
  (for _array_element _outactors
    (if (`self.ActorHasTag` _array_element _ball_type)
      (if (`self.ActorHasTag` _array_element (`self.Left Or Right`))
        (`KismetArrayLibrary.Array_AddUnique` (`self.SplinesSelected`) _array_element)
        (`self.StartMoving`)
        (return _ball_type)))))

(fn `Choose Pitcher Type`
  (params (`Pitcher Type` :type Name))
  (returns (`Pitcher Name` :type Name))
  (bind _pitcher_type (`self.Pitcher Type`))
  (set `self.Pitcher Type` `Pitcher Type`)
  (bind _outactors (`GameplayStatics.GetAllActorsOfClass` "/Game/team09/character/BP_BaseCharacter.BP_BaseCharacter_C"))
  (for _array_element _outactors
    (if (`self.ActorHasTag` _array_element (`self.Pitcher Type`))
      (set `self.CharacterSelected` _array_element)
      (`KismetSystemLibrary.PrintString` (`KismetStringLibrary.Conv_NameToString` _pitcher_type))
      (return _pitcher_type))))

(fn `Launch`
  (`PrimitiveComponent.AddImpulse` (`self.StaticMesh`) (* (`self.GetActorForwardVector` self) 2000.0) "None" true))

(fn `UserConstructionScript`)