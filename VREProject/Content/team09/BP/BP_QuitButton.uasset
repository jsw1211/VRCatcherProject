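; BP_QuitButton is a physical in-world button that quits the game when pressed.
; Its ButtonComponent's ButtonPressed event calls QuitGame.
; InvisibleEvent and VisibleEvent hide or show the mesh, button component and text render, also toggling collision on the mesh and button.
; The construction script only calls its parent, and NewFunction is empty.
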(event `Invisible Event`
  (bind _staticmesh (`self.StaticMesh`))
  (bind _buttoncomponent (`self.ButtonComponent`))
  (`SceneComponent.SetVisibility` _staticmesh false false)
  (`PrimitiveComponent.SetCollisionEnabled` _staticmesh "NoCollision")
  (`SceneComponent.SetVisibility` _buttoncomponent false false)
  (`PrimitiveComponent.SetCollisionEnabled` _buttoncomponent "NoCollision")
  (`SceneComponent.SetVisibility` (`self.TextRender`) false false))

(event `Visible Event`
  (bind _staticmesh (`self.StaticMesh`))
  (bind _buttoncomponent (`self.ButtonComponent`))
  (`SceneComponent.SetVisibility` _staticmesh true false)
  (`PrimitiveComponent.SetCollisionEnabled` _staticmesh "QueryAndPhysics")
  (`SceneComponent.SetVisibility` _buttoncomponent true false)
  (`PrimitiveComponent.SetCollisionEnabled` _buttoncomponent "QueryAndPhysics")
  (`SceneComponent.SetVisibility` (`self.TextRender`) true false))

(event `self.ButtonComponent.ButtonPressed`
  (params (ButtonState :type Boolean))
  (`KismetSystemLibrary.QuitGame` null "Quit"))

(fn `NewFunction`)

(fn `UserConstructionScript`
  (`parent.UserConstructionScript`))