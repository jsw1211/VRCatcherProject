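; BP_RestartButton is an in-world Restart button that clears the game result shown by BP_GameResultManager.
; Pressing its ButtonComponent, or the V key, finds the manager with GetActorOfClass and calls InvisibleButtons and ClearResult.
; VisibleEvent and InvisibleEvent toggle visibility and collision of the mesh and button along with the text's visibility.
; Showing it also sets a red OnColor and the "Restart" label.
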(event `Invisible Event`
  (bind _staticmesh (`self.StaticMesh`))
  (bind _buttoncomponent (`self.ButtonComponent`))
  (`SceneComponent.SetVisibility` _staticmesh false false)
  (`PrimitiveComponent.SetCollisionEnabled` _staticmesh "NoCollision")
  (`SceneComponent.SetVisibility` _buttoncomponent false false)
  (`PrimitiveComponent.SetCollisionEnabled` _buttoncomponent "NoCollision")
  (`SceneComponent.SetVisibility` (`self.TextRender`) false false))

(event `Visible Event`
  (bind _staticmesh (`self.StaticMesh`))
  (bind _buttoncomponent (`self.ButtonComponent`))
  (bind _textrender (`self.TextRender`))
  (`SceneComponent.SetVisibility` _staticmesh true false)
  (`PrimitiveComponent.SetCollisionEnabled` _staticmesh "QueryAndPhysics")
  (`SceneComponent.SetVisibility` _buttoncomponent true false)
  (`PrimitiveComponent.SetCollisionEnabled` _buttoncomponent "QueryAndPhysics")
  (`SceneComponent.SetVisibility` _textrender true false)
  (set `/Game/Platform/Interaction/Button/ButtonComponent.OnColor` (struct :`R` 1.0 :`A` 1.0) _buttoncomponent)
  (`TextRenderComponent.K2_SetText` _textrender (`KismetTextLibrary.Conv_StringToText` "Restart")))

(event `Key|V`
  (params (Key :type "Key Structure"))
  (:`Pressed`
    (bind _returnvalue (`GameplayStatics.GetActorOfClass` "/Game/team09/BP/BP_GameResultManager.BP_GameResultManager_C" :!label _label))
    (`/Game/team09/BP/BP_GameResultManager.Invisible Buttons` _returnvalue)
    (`/Game/team09/BP/BP_GameResultManager.ClearResult` _returnvalue)))

(event `self.ButtonComponent.ButtonPressed`
  (params (ButtonState :type Boolean))
  (goto _label))

(event `self.ReceiveBeginPlay`
  (`self.EnableInput` (`GameplayStatics.GetPlayerController` 0)))

(fn `NewFunction`)

(fn `UserConstructionScript`
  (`parent.UserConstructionScript`))