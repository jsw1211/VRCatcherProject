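; BP_Catcher handles left-hand catcher's mitt input, apparently as a VR character, animating the glove to close and open.
; Left primary grip casts GraspingHandLeft to BP_Hand and plays the Glove's closing animation on press, opening on release or cancel.
; Grip and use-held-object inputs also set pressed flags, unread here, and print debug text on press.
; The J key plays the closing animation alone.
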(event `self.ReceiveTick`
  (params (DeltaSeconds :type "Float (single-precision)"))
  (`parent.ReceiveTick` DeltaSeconds))

(event `EnhancedInput|/Game/Platform/Input/Actions/UseHeldObjectLeft`
  (params (ActionValue :type Boolean) (ElapsedSeconds :type "Float (double-precision)") (TriggeredSeconds :type "Float (double-precision)") (InputAction :type "InputAction Object Reference" :default "/Game/Platform/Input/Actions/UseHeldObjectLeft.UseHeldObjectLeft"))
  (:`Started`
    (set `self.bUseHeldObjectPressed` true)
    (`KismetSystemLibrary.PrintString` "Held"))
  (:`Canceled`
    (set `self.bUseHeldObjectPressed` false :!label _label))
  (:`Completed`
    (goto _label)))

(event `EnhancedInput|/Game/Platform/Input/Actions/PrimaryGripLeft`
  (params (ActionValue :type Boolean) (ElapsedSeconds :type "Float (double-precision)") (TriggeredSeconds :type "Float (double-precision)") (InputAction :type "InputAction Object Reference" :default "/Game/Platform/Input/Actions/PrimaryGripLeft.PrimaryGripLeft"))
  (bind _graspinghandleft (`self.GraspingHandLeft`))
  (:`Started`
    (set `self.bPrimaryGripPressed` true)
    (`KismetSystemLibrary.PrintString` "Pri")
    (bind _asbp_hand (cast `/Game/team09/BP/BP_Hand` _graspinghandleft))
    (`SkeletalMeshComponent.PlayAnimation` (`/Game/team09/BP/BP_Hand.Glove` _asbp_hand) "/Game/team09/Asset/glove/catchermitt_anim_closing_Anim.catchermitt_anim_closing_Anim" false))
  (:`Canceled`
    (set `self.bPrimaryGripPressed` false :!label _label_2)
    (bind _asbp_hand_2 (cast `/Game/team09/BP/BP_Hand` _graspinghandleft))
    (`SkeletalMeshComponent.PlayAnimation` (`/Game/team09/BP/BP_Hand.Glove` _asbp_hand_2) "/Game/team09/Asset/glove/catchermitt_anim_opening_Anim.catchermitt_anim_opening_Anim" false))
  (:`Completed`
    (goto _label_2)))

(event `Key|J`
  (params (Key :type "Key Structure"))
  (:`Pressed`
    (bind _asbp_hand (cast `/Game/team09/BP/BP_Hand` (`self.GraspingHandLeft`)))
    (`SkeletalMeshComponent.PlayAnimation` (`/Game/team09/BP/BP_Hand.Glove` _asbp_hand) "/Game/team09/Asset/glove/catchermitt_anim_closing_Anim.catchermitt_anim_closing_Anim" false)))

(fn `UserConstructionScript`
  (`parent.UserConstructionScript`))