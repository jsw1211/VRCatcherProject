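; BP_DifficultyButton is a button Blueprint that toggles a pro-mode difficulty flag and shows an On/Off label.
; Each ButtonPressed event from ButtonComponent prints a debug message, flips IsProMod and updates the TextRender.
; The label reads On when IsProMod becomes false and Off when it becomes true.
; The flag is only set locally, and NewFunction is an empty stub.
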(event `self.ButtonComponent.ButtonPressed`
  (params (ButtonState :type Boolean))
  (bind _textrender (`self.TextRender`))
  (`KismetSystemLibrary.PrintText` "ButtonPressed")
  (if (`self.IsProMod`)
    (`TextRenderComponent.K2_SetText` _textrender (`self.On`))
    (set `self.IsProMod` false)
    (else
      (`TextRenderComponent.K2_SetText` _textrender (`self.Off`))
      (set `self.IsProMod` true))))

(fn `NewFunction`)

(fn `UserConstructionScript`
  (`parent.UserConstructionScript`))