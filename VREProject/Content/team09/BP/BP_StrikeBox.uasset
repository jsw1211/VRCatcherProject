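; BP_StrikeBox is a baseball strike zone that calls pitches as Strike or Ball and shows the result as text.
; Overlaps of BP_BaseballBall with two collision volumes set CallState, with an active Strike blocking Ball, and the text clears after a delay.
; UpdateCatchText separately shows Catch or Miss from CatchState, with no caller in this graph.
; The construction script builds the visible zone as a grid of scaled mesh tiles.
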(event `self.ReceiveTick`
  (params (DeltaSeconds :type "Float (single-precision)")))

(event `self.StrikeCollision.OnComponentBeginOverlap`
  (params (OverlappedComponent :type "PrimitiveComponent Object Reference") (OtherActor :type "Actor Object Reference") (OtherComp :type "PrimitiveComponent Object Reference") (OtherBodyIndex :type Integer) (bFromSweep :type Boolean) (SweepResult :type "HitResult Structure (by ref)"))
  (cast `/Game/team09/BP/BP_BaseballBall` OtherActor)
  (set `self.CallState` "NewEnumerator1")
  (`self.UpdateStrikeText`)
  (`KismetSystemLibrary.Delay` (`self.TextDelay`))
  (set `self.CallState` "NewEnumerator0")
  (`self.UpdateStrikeText`))

(event `self.BallCollision.OnComponentBeginOverlap`
  (params (OverlappedComponent :type "PrimitiveComponent Object Reference") (OtherActor :type "Actor Object Reference") (OtherComp :type "PrimitiveComponent Object Reference") (OtherBodyIndex :type Integer) (bFromSweep :type Boolean) (SweepResult :type "HitResult Structure (by ref)"))
  (cast `/Game/team09/BP/BP_BaseballBall` OtherActor)
  (if (not (`|EnumEquality` (`self.CallState`) "NewEnumerator1"))
    (set `self.CallState` "NewEnumerator2")
    (`self.UpdateStrikeText`)
    (`KismetSystemLibrary.Delay` (`self.TextDelay`))
    (set `self.CallState` "NewEnumerator0")
    (`self.UpdateStrikeText`)))

(event `UpdateStrikeText`
  (bind _strike_text (`self.Strike_Text`))
  (switch `/Game/team09/BP/Enum/BP_StrikeState` (`self.CallState`)
    (:`NewEnumerator0`
      (`TextRenderComponent.K2_SetText` _strike_text (`self.Empty`)))
    (:`NewEnumerator1`
      (`TextRenderComponent.K2_SetText` _strike_text (`self.Strike`)))
    (:`NewEnumerator2`
      (`TextRenderComponent.K2_SetText` _strike_text (`self.Ball`)))))

(event `UpdateCatchText`
  (bind _catch_text (`self.Catch_Text`))
  (switch `/Game/team09/BP/Enum/BP_CatchState` (`self.CatchState`)
    (:`NewEnumerator0`
      (`TextRenderComponent.K2_SetText` _catch_text (`self.Catch`)))
    (:`NewEnumerator1`
      (`TextRenderComponent.K2_SetText` _catch_text (`self.Miss`)))))

(fn `UserConstructionScript`
  (bind _grid (`self.Grid`))
  (for _index (range (+ _grid 1))
    (for _index_2 (range (+ _grid 1))
      (bind _returnvalue (`AddComponent|NODE_AddStaticMeshComponent-0` :`self` (`ActorComponent.GetOwner` (`self.Strike Zone`))))
      (`StaticMeshComponent.SetStaticMesh` _returnvalue (`StaticMeshComponent.StaticMesh` (`self.Strike Zone`)))
      (`PrimitiveComponent.SetMaterial` _returnvalue 0 "/Game/team09/BP/M_StrikeZone.M_StrikeZone")
      (`SceneComponent.K2_SetRelativeLocation` _returnvalue (`KismetMathLibrary.MakeVector` 0.0 (`KismetMathLibrary.Conv_IntToDouble` (* _index 32)) (`KismetMathLibrary.Conv_IntToDouble` (* _index_2 50))) false false)
      (`SceneComponent.SetRelativeScale3D` _returnvalue (0.01 0.31 0.49)))))